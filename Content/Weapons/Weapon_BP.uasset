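; Weapon actor that toggles between a gun and a sword, tracked by an IsGun flag.
; ChangeWeapon flips the flag and swaps the mesh between a sphere for the gun and a blue-light sword.
; In gun mode, Shoot fires a long forward visibility line trace with debug drawing, but the hit result is unused.
; BeginPlay sets the PhysicsHandle linear stiffness, and SwapWeapon is an empty stub.
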(event EventBeginPlay
  (Class|PhysicsHandleComponent|SetLinearStiffness (Variables|Default|GetPhysicsHandle) 1.0))

(event Collision|EventActorBeginOverlap
  (params (OtherActor :type Actor%20Object%20Reference)))

(event EventTick
  (params (DeltaSeconds :type Float%20%28single-precision%29)))

(fn ConstructionScript)

(fn Shoot
  (bind _returnvalue (Transformation|GetActorLocation))
  (if (Variables|Default|GetIs_Gun)
    (Collision|LineTraceByChannel _returnvalue (+ _returnvalue (* (Math|Rotator|GetRotationXVector (Transformation|GetActorRotation)) 2.5e+04)) "TraceTypeQuery1" false 0 "ForDuration")))

(fn ChangeWeapon
  (bind _weapon_mesh (Variables|Default|GetWeapon_Mesh))
  (if (Variables|Default|GetIs_Gun)
    (Variables|Default|SetIs_Gun false)
    (Components|StaticMesh|SetStaticMesh _weapon_mesh "/Game/Assets/bluelight_sword_Cube.bluelight_sword_Cube")
    (else
      (Variables|Default|SetIs_Gun true)
      (Components|StaticMesh|SetStaticMesh _weapon_mesh "/Engine/EngineMeshes/Sphere.Sphere"))))

(fn SwapWeapon)